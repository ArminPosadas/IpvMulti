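; BP_LaunchPad2 is a launch pad that throws BP_ThirdPersonCharacter along the pad's facing direction.
; Overlapping LaunchCol calls LaunchCharacter with the forward vector scaled by LaunchStrenght and a fixed upward Z, overriding current velocity.
; When RotationYaw is enabled, Tick sets the absolute yaw from a sine of game time, so the launch direction swings back and forth.
; An unconnected debug line draw never runs.
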(event `self.ReceiveTick`
  (params (DeltaSeconds :type "Float (single-precision)"))
  (if (`self.RotationYaw`)
    (`self.K2_SetActorRotation` (`KismetMathLibrary.MakeRotator` 0.0 0.0 (* (`KismetMathLibrary.Sin` (* (`KismetSystemLibrary.GetGameTimeInSeconds`) (`self.RotationSpeed`))) (`self.RotationAmplitude`))))))

(event `self.LaunchCol.OnComponentBeginOverlap`
  (params (OverlappedComponent :type "PrimitiveComponent Object Reference") (OtherActor :type "Actor Object Reference") (OtherComp :type "PrimitiveComponent Object Reference") (OtherBodyIndex :type Integer) (bFromSweep :type Boolean) (SweepResult :type "HitResult Structure (by ref)"))
  (bind _asbp_third_person_character (cast `/Game/ThirdPerson/Blueprints/BP_ThirdPersonCharacter` OtherActor))
  (`Character.LaunchCharacter` _asbp_third_person_character (`KismetMathLibrary.MakeVector` (.x (* (`self.GetActorForwardVector`) (`self.LaunchStrenght`))) (.y (* (`self.GetActorForwardVector`) (`self.LaunchStrenght`))) 800.0) true true))

(fn `UserConstructionScript`)