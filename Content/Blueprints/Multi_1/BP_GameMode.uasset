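; Game mode for the Multi_1 Blueprints that opens the main menu and handles the camera change when a mission completes.
; On BeginPlay it gives the first player UI-only input with a visible cursor and adds the main menu widget to the viewport.
; OnMissionCompleted blends the completing pawn's controller view to the first BP_EspectatorView actor with a cubic blend.
; A player-won widget branch exists but is disconnected.
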(event `self.ReceiveBeginPlay`
  (bind _returnvalue (`GameplayStatics.GetPlayerController` 0))
  (`WidgetBlueprintLibrary.SetInputMode_UIOnlyEx` _returnvalue null)
  (set `PlayerController.bShowMouseCursor` true _returnvalue)
  (bind _returnvalue_2 (`|CreateWidget` "/Game/Blueprints/Multi_2/MainMenuWidget.MainMenuWidget_C" _returnvalue))
  (`UserWidget.AddToViewport` _returnvalue_2 0))

(event `self.OnMissionCompleted`
  (params (Pawn :type "Pawn Object Reference"))
  (bind _asplayer_controller (cast `PlayerController` (`Pawn.GetController` Pawn)))
  (bind _outactors (`GameplayStatics.GetAllActorsOfClass` "/Game/Blueprints/Multi_1/BP_EspectatorView.BP_EspectatorView_C"))
  (`PlayerController.SetViewTargetWithBlend` _asplayer_controller (`|GetArrayItem` _outactors) 1.0 "VTBlend_Cubic" 0.0 false))

(fn `UserConstructionScript`)