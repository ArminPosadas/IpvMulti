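; BP_LaunchPad3 is a launch pad actor that moves along its forward vector when its MoveLaunchPad event is called.
; The event slows a timeline's play rate to a small fraction, then plays it to drive SetActorLocation without sweeping.
; Each update lerps from the current location toward a point a fixed distance ahead of it, so movement compounds instead of interpolating between fixed endpoints.
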(event `self.ReceiveBeginPlay`)

(event `MoveLaunchPad`
  (`TimelineComponent.SetPlayRate` (`self.Timeline_Move_LaunchPad`) (/ 1.0 100.0))
  (bind (_direction _alpha) (`Timeline|Timeline_Move_LaunchPad`)
    (:`Update`
      (`self.K2_SetActorLocation` (`KismetMathLibrary.VLerp` (`self.K2_GetActorLocation`) (+ (`self.K2_GetActorLocation`) (* (`KismetMathLibrary.GetForwardVector` (`self.K2_GetActorRotation`)) 400.0)) _alpha)))))

(fn `UserConstructionScript`)