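; BP_PunchBox is an actor that punches out along its forward vector and retracts, repeating once triggered.
; PunchingBlock enters a FlipFlop that alternately plays and reverses a timeline, whose alpha offsets the location saved at BeginPlay by MoveDistance, without sweeping.
; Each timeline update restarts a retriggerable Cooldown delay that loops back into the FlipFlop, so the direction flips once updates stop for that duration.
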(event `self.ReceiveBeginPlay`
  (set `self.OriginalPosition` (`self.K2_GetActorLocation`)))

(event `Punching Block`
  (`/Engine/EditorBlueprintResources/StandardMacros.FlipFlop` :!label _label
    (:`A`
      (bind (_direction _alpha) (`Timeline|Punching_Timeline` :!label _label_2)
        (:`Update`
          (`self.K2_SetActorLocation` (+ (`self.OriginalPosition`) (* (* (`self.GetActorForwardVector`) _alpha) (`self.MoveDistance`))))
          (`KismetSystemLibrary.RetriggerableDelay` (`self.Cooldown`))
          (goto _label))))
    (:`B`
      (goto _label_2 :!via `Reverse`))))

(fn `UserConstructionScript`)