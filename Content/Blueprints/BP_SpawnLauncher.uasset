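; BP_SpawnLauncher is a spawner actor that produces moving BP_LaunchPad3 launch pads at its own transform.
; BeginPlay starts a looping timer, and the SpawnLaunchPad event creates each pad only on the server.
; Each new pad is told to move through MoveLaunchPad and is given a lifespan so it is destroyed automatically.
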(event `self.ReceiveBeginPlay`
  (`KismetSystemLibrary.K2_SetTimerDelegate` (`|CreateDelegate` :!event `SpawnLaunchPad`) 2.0 true))

(event `SpawnLaunchPad`
  (if (`KismetSystemLibrary.IsServer`)
    (bind _returnvalue (`|SpawnActorFromClass` "/Game/Blueprints/BP_LaunchPad3.BP_LaunchPad3_C" (`self.GetTransform`) "Undefined" "MultiplyWithRoot" null null))
    (bind _output_get (set `self.LaunchPad` _returnvalue))
    (`/Game/Blueprints/BP_LaunchPad3.MoveLaunchPad` _output_get)
    (`self.SetLifeSpan` (`self.LaunchPad`) (`self.In Lifespan`))))

(fn `UserConstructionScript`)