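; BP_LaunchForce is an actor that moves along its forward vector from its starting position, scaled by MoveDistance.
; BeginPlay stores the origin, and Tick calls Movement every frame while CanMove is set.
; Movement's FlipFlop alternates playing and reversing a Timeline whose Alpha sets the location without sweep.
; The Timeline's Update and Finished outputs both feed back into that FlipFlop, and no launch force is applied.
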(event `self.ReceiveBeginPlay`
  (set `self.OriginalPosition` (`self.K2_GetActorLocation`)))

(event `Movement`
  (`/Engine/EditorBlueprintResources/StandardMacros.FlipFlop` :!label _label
    (:`A`
      (bind (_direction _alpha) (`Timeline|Timeline` :!label _label_2)
        (:`Update`
          (`self.K2_SetActorLocation` (+ (`self.OriginalPosition`) (* (* (`self.GetActorForwardVector`) _alpha) (`self.MoveDistance`))))
          (goto _label))
        (:`Finished`
          (goto _label))))
    (:`B`
      (goto _label_2 :!via `Reverse`))))

(event `self.ReceiveTick`
  (params (DeltaSeconds :type "Float (single-precision)"))
  (if (`self.Can Move`)
    (`self.Movement`)))

(fn `UserConstructionScript`)