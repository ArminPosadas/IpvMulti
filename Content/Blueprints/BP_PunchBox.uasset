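; BP_PunchBox is a block that punches back and forth along the world X axis.
; BeginPlay caches its starting X, and the PunchingBlock event plays or reverses a timeline based on IsMovingRight.
; Timeline updates offset X by Alpha times MoveDistance without sweeping, then enter a Cooldown delay.
; A FlipFlop after the delay sets the direction flag and loops back to the branch, sustaining the motion.
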(event `self.ReceiveBeginPlay`
  (set `self.OriginalX` (.x (`self.K2_GetActorLocation`))))

(event `Punching Block`
  (if (`self.IsMovingRight`) :!label _label
    (bind (_direction _alpha) (`Timeline|Punching_Timeline` :!label _label_2)
      (:`Update`
        (`self.K2_SetActorLocation` (`KismetMathLibrary.MakeVector` (+ (`self.OriginalX`) (* _alpha (`self.MoveDistance`))) (.y (`self.K2_GetActorLocation`)) (.z (`self.K2_GetActorLocation`))))
        (`KismetSystemLibrary.Delay` (`self.Cooldown`))
        (`/Engine/EditorBlueprintResources/StandardMacros.FlipFlop`
          (:`A`
            (set `self.IsMovingRight` false)
            (goto _label))
          (:`B`
            (set `self.IsMovingRight` true)
            (goto _label)))))
    (else
      (goto _label_2 :!via `Reverse`))))

(fn `UserConstructionScript`)