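; BP_Trap is a trap actor meant to punch back and forth along the world X axis.
; BeginPlay only caches the starting X position.
; A disconnected movement graph, which never runs, offsets X by timeline alpha times MoveDistance, playing or reversing according to IsMovingRight.
; That graph's timeline update also triggers a cooldown Delay and FlipFlop that sets the direction and loops back.
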(event `self.ReceiveBeginPlay`
  (set `self.OriginalX` (.x (`self.K2_GetActorLocation`))))

(fn `UserConstructionScript`)